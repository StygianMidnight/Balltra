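; BP_PlayerStats is an actor that keeps counters for balls the player hits: left, right and total.
; The TrackBallHit event takes a hit side and increments one counter per call.
; "Left" raises the left count and any other value raises only the total.
; The right counter is unreachable because its branch repeats the "Left" comparison.
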(event `TrackBallHit`
  (params (HitSide :type String))
  (if (== HitSide "Left")
    (bind _result (`/Engine/EditorBlueprintResources/StandardMacros.IncrementInt` (`self.BallsHit_Left`))
      (:`  `
        (set `self.BallsHit_Left` _result)))
    (elif (== HitSide "Left")
      (bind _result_2 (`/Engine/EditorBlueprintResources/StandardMacros.IncrementInt` (`self.BallsHit_Right`))
        (:`  `
          (set `self.BallsHit_Right` _result_2)))
      (else
        (bind _result_3 (`/Engine/EditorBlueprintResources/StandardMacros.IncrementInt` (`self.TotalBallsHit`))
          (:`  `
            (set `self.TotalBallsHit` _result_3)))))))

(fn `UserConstructionScript`)